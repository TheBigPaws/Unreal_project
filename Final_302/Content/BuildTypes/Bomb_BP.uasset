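; Bomb actor that blows up destroyable build cubes within its blast radius.
; While IsReal is set, Tick counts up a short fuse, then destroys overlapping TestBuildCubeBP actors flagged Destroyable, spawns an explosion emitter and destroys itself.
; SetCollisions toggles physics simulation on the main mesh and collision on the mesh, fuse and top together.
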(event EventBeginPlay)

(event Collision|EventActorBeginOverlap
  (params (OtherActor :type Actor%20Object%20Reference)))

(event EventTick
  (params (DeltaSeconds :type Float%20%28single-precision%29))
  (if (Variables|Default|GetisReal)
    (bind _output_get (Variables|Default|SetLifeTime (+ DeltaSeconds (Variables|Default|GetLifeTime))))
    (if (> _output_get 2.0)
      (for _array_element (Collision|GetOverlappingActors (Variables|Default|GetBlastRadius) "/Game/BuildTypes/testBuildCubeBP.testBuildCubeBP_C" :!class /Script/Engine.PrimitiveComponent)
        (bind _astest_build_cube_bp (Utilities|Casting|CastTotestBuildCubeBP _array_element))
        (if (Variables|/Game/BuildTypes/testBuildCubeBP.testBuildCubeBP_C|GetDestroyable _astest_build_cube_bp)
          (Actor|DestroyActor _array_element)))
      (Effects|SpawnEmitteratLocation "/Game/StarterContent/Particles/P_Explosion.P_Explosion" (Transformation|GetActorLocation))
      (Actor|DestroyActor))))

(fn ConstructionScript)

(fn SetCollisions
  (params (setTo :type Boolean))
  (bind _fuse (Variables|Default|Getfuse))
  (bind _bombtop (Variables|Default|GetBombTop))
  (bind _staticmeshcomponent (Variables|Debug|GetStaticMeshComponent))
  (bind _staticmeshcomponent_2 (Variables|Debug|GetStaticMeshComponent))
  (if setTo
    (Physics|SetSimulatePhysics _staticmeshcomponent_2 true)
    (Collision|SetCollisionEnabled _fuse "QueryAndPhysics")
    (Collision|SetCollisionEnabled _bombtop "QueryAndPhysics")
    (Collision|SetCollisionEnabled _staticmeshcomponent "QueryAndPhysics")
    (else
      (Physics|SetSimulatePhysics _staticmeshcomponent_2 false)
      (Collision|SetCollisionEnabled _fuse "NoCollision")
      (Collision|SetCollisionEnabled _bombtop "NoCollision")
      (Collision|SetCollisionEnabled _staticmeshcomponent "NoCollision"))))